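; Player controller that creates the main HUD widget and drives a top-down character with movement, attack and cursor aiming.
; On possess it stores the BP_PlayerCharacter in BP_PlayerState, and all input reaches the character through that reference.
; Movement follows fixed world axes.
; Each tick it traces under player 0's cursor and calls LookAt with authority or ClientLookAt on remote.
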(event EventBeginPlay
  (bind _returnvalue (UserInterface|CreateWidget "/Game/uIO/Maps/W_Main.W_Main_C"))
  (UserInterface|Viewport|AddtoViewport _returnvalue 0))

(event EventTick
  (params (DeltaSeconds :type Float%20%28single-precision%29))
  (bind _returnvalue (Game|GetPlayerController 0))
  (bind _hitresult (Game|Player|GetHitResultUnderCursorbyChannel _returnvalue "TraceTypeQuery1" true))
  (bind _location (Collision|BreakHitResult _hitresult))
  (Networking|SwitchHasAuthority
    (:Authority
      (bind _asbp_player_state (Utilities|Casting|CastToBP_PlayerState (Variables|GetPlayerState)))
      (Default|Lookat (Variables|/Game/uIO/Core/BP_PlayerState.BP_PlayerState_C|GetPlayerCharacter _asbp_player_state) _location))
    (:Remote
      (bind _asbp_player_state_2 (Utilities|Casting|CastToBP_PlayerState (Variables|GetPlayerState)))
      (Default|ClientLookat (Variables|/Game/uIO/Core/BP_PlayerState.BP_PlayerState_C|GetPlayerCharacter _asbp_player_state_2) _location))))

(event EventPossess
  (params (PossessedPawn :type Pawn%20Object%20Reference))
  (bind _asbp_player_character (Utilities|Casting|CastToBP_PlayerCharacter PossessedPawn))
  (bind _asbp_player_state (Utilities|Casting|CastToBP_PlayerState (Variables|GetPlayerState)))
  (Variables|/Game/uIO/Core/BP_PlayerState.BP_PlayerState_C|SetPlayerCharacter _asbp_player_state _asbp_player_character)
  (Development|PrintString "Hello"))

(event Input|ActionEvents|InputActionAttack
  (params (Key :type Key%20Structure))
  (:Pressed
    (bind _asbp_player_state (Utilities|Casting|CastToBP_PlayerState (Variables|GetPlayerState)))
    (Default|Attack (Variables|/Game/uIO/Core/BP_PlayerState.BP_PlayerState_C|GetPlayerCharacter _asbp_player_state))))

(event Input|AxisEvents|InputAxisMoveForward
  (params (AxisValue :type Float%20%28single-precision%29))
  ;[1 1 1] 移动
  (if (!= AxisValue 0.0)
    (bind _asbp_player_state (Utilities|Casting|CastToBP_PlayerState (Variables|GetPlayerState)))
    (Pawn|Input|AddMovementInput (Variables|/Game/uIO/Core/BP_PlayerState.BP_PlayerState_C|GetPlayerCharacter _asbp_player_state) "1.000000, 0, 0" AxisValue false)))

(event Input|AxisEvents|InputAxisMoveRight
  (params (AxisValue :type Float%20%28single-precision%29))
  ;[1 1 1] 移动
  (if (!= AxisValue 0.0)
    (bind _asbp_player_state (Utilities|Casting|CastToBP_PlayerState (Variables|GetPlayerState)))
    (Pawn|Input|AddMovementInput (Variables|/Game/uIO/Core/BP_PlayerState.BP_PlayerState_C|GetPlayerCharacter _asbp_player_state) "0.000000,1.000000, 0" AxisValue false)))

(fn ConstructionScript)