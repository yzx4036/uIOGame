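; Game mode that spawns the players, AI monsters and blocks, and feeds characters into BP_GameState.
; BeginPlay caches the game state, seeds its player list with existing characters and calls InitBlock, whose 200-range loop returns after the first block spawn attempt.
; PostLogin spawns, possesses and registers a character at a random navigable point.
; Tick uses a Delay to spawn and register a behavior-tree monster about every ten seconds.
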(event EventBeginPlay
  (bind _asbp_game_state (Utilities|Casting|CastToBP_GameState (Game|GetGameState)))
  (Variables|Default|SetMyGameState _asbp_game_state)
  (bind _outactors (Actor|GetAllActorsOfClass "/Game/uIO/Character/BP_CharacterBase.BP_CharacterBase_C"))
  (Variables|/Game/uIO/Core/BP_GameState.BP_GameState_C|SetPlayerList (Variables|Default|GetMyGameState) _outactors)
  (CallFunction|InitBlock))

(event EventPostLogin
  (params (NewPlayer :type Player%20Controller%20Object%20Reference))
  (bind _returnvalue (Game|SpawnActorfromClass "/Game/uIO/Character/BP_PlayerCharacter.BP_PlayerCharacter_C" (Math|Conversions|ToTransform(Vector) (.RandomLocation (Class|NavigationSystemV1|GetRandomPointinNavigableRadius (Math|Vector|MakeVector 0.0 0.0 0.0) 1e+03 0 0))) "AdjustIfPossibleButAlwaysSpawn" 0 0))
  (Pawn|Possess NewPlayer _returnvalue)
  (bind _asbp_game_state (Utilities|Casting|CastToBP_GameState (Game|GetGameState)))
  (Default|SetPlayer _asbp_game_state _returnvalue))

(event EventTick
  (params (DeltaSeconds :type Float%20%28single-precision%29))
  (Utilities|FlowControl|Delay 1e+01)
  (bind _returnvalue (AI|SpawnAIFromClass "/Game/uIO/Character/BP_Monster.BP_Monster_C" "/Game/uIO/AI/BT_Enemy.BT_Enemy" (.RandomLocation (AI|Navigation|GetRandomReachablePointinRadius (Math|Vector|MakeVector 0.0 0.0 0.0) 1e+03 0 0)) "0, 0, 0" false))
  (bind _asbp_character_base (Utilities|Casting|CastToBP_CharacterBase _returnvalue))
  (Default|SetPlayer (Variables|Default|GetMyGameState) _asbp_character_base))

(fn ConstructionScript)

(fn InitBlock
  (for _index (range 0 200)
    (Game|SpawnActorfromClass "/Game/uIO/Block/BP_Block.BP_Block_C" (Math|Transform|MakeTransform (.RandomLocation (AI|Navigation|GetRandomReachablePointinRadius (Math|Vector|MakeVector 0.0 0.0 0.0) 5e+03 0 0))) "AdjustIfPossibleButDontSpawnIfColliding" 0 0)
    (return)))