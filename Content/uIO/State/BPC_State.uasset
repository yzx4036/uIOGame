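; BPC_State is a Blueprint component that stores stats in a States map from a state key to an S_State struct holding Current, Min and Max.
; GetState and SetState read and write map entries, while ModifyState adds a delta to Current and clamps it between Min and Max.
; After every modification, whichever state changed, it calls OnDeath if the state keyed by the NewEnumerator0 enum entry sits at its minimum.
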(event EventBeginPlay)

(event EventTick
  (params (DeltaSeconds :type Float%20%28single-precision%29)))

(fn GetState
  (params (Key :type EState%20Enum :default "NewEnumerator0"))
  (return (.Value (Utilities|Map|Find (Variables|Default|GetStates) Key))))

(fn SetState
  (params (StateID :type EState%20Enum%20%28by%20ref%29 :default "NewEnumerator0") (StateInfo :type S%20State%20Structure%20%28by%20ref%29))
  (Utilities|Map|Add (Variables|Default|GetStates) StateID StateInfo)
  (return))

(fn ModifyState
  (params (State :type EState%20Enum :default "NewEnumerator0") (by :type Integer))
  (bind _value (CallFunction|GetState "NewEnumerator0"))
  (bind _value_2 (CallFunction|GetState State))
  (bind (_min _max _current) (Utilities|Struct|BreakSState _value_2))
  (bind _structout (Utilities|Struct|SetmembersinSState _value_2 (Math|Integer|Clamp(Integer) (+ _current by) _min _max)))
  (CallFunction|SetState State _structout)
  (if (== (.min _value) (.current _value))
    (Default|CallOnDeath)
    (return)
    (else
      (return))))